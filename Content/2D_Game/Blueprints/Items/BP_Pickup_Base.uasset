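; Base Blueprint for 2D game pickup items, exposing interaction functions and item text.
; On BeginPlay it caches the 2D game mode, whose HUD widget Interact uses to show the item name before destroying the actor.
; GetPicked supplies that display name, while a separate ItemPicked returns name and description for inventory text.
; GetWidgetType returns a fixed type, ShowNextLine always returns false, and FinishInteraction is empty.
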(event `self.ReceiveBeginPlay`
  (bind _as2d_game_mode (cast `/Game/2D_Game/Blueprints/2D_GameMode` (`GameplayStatics.GetGameMode`)))
  (set `self.GameMode` _as2d_game_mode))

(event `/Game/2D_Game/Blueprints/Interfaces/BPI_Interaction.FinishInteraction`)

(fn `GetPicked`
  (returns (ItemName :type String))
  ;[1 1 1] 好像只是用来显示物品拾起信息，不参与inventory
  (return (`self.ItemName`)))

(fn `GetWidgetType`
  (returns (WidgetType :type "/Game/2D_Game/Widgets/EWidgetType Enum"))
  (return "NewEnumerator0"))

(fn `Interact`
  (params (Insitigator :type "/Game/2D_Game/Blueprints/Characters/MainCharacter/PlayerModel_BP Object Reference"))
  (bind _itemname (`self.GetPicked`))
  (`/Game/2D_Game/Widgets/WBP_MainHUD.SetItemText` (`/Game/2D_Game/Blueprints/2D_GameMode.HUDWidget` (`self.GameMode`)) _itemname self)
  (`self.K2_DestroyActor`)
  (return))

(fn `ItemPicked`
  (returns (ItemName :type String) (ItemDescription :type String))
  (bind _itemname (`self.ItemName`))
  ;[1 1 1] 参与inventory文字变量
  (`KismetSystemLibrary.PrintString` _itemname)
  (return _itemname (`self.Item Description`)))

(fn `ShowNextLine`
  (returns (HasNextLine :type Boolean))
  (return false))

(fn `UserConstructionScript`)