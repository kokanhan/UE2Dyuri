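; Player character Blueprint for a 2D game, handling Enhanced Input movement, interaction and inventory toggling.
; Interaction scans InteractCheck overlaps, adds BPI_Item pickups to the inventory component and sends an interact message, remembering the target.
; While interaction is locked, movement is ignored and the interact key instantly reveals or advances dialogue, unlocking when lines run out.
; Dialogue, inventory and timed item-message UI are reached through the GameMode's HUD widget.
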(event `self.ReceiveBeginPlay`
  (`|ExecutionSequence`
    (:`then_0`
      (`EnhancedInputSubsystemInterface.AddMappingContext` (pcsubsystem `EnhancedInputLocalPlayerSubsystem` (`GameplayStatics.GetPlayerController` 0)) "/Game/2D_Game/Inputs/IMC_Player.IMC_Player" 0 (struct)))
    (:`then_1`
      (bind _as2d_game_mode (cast `/Game/2D_Game/Blueprints/2D_GameMode` (`GameplayStatics.GetGameMode`)))
      (set `self.GameMode` _as2d_game_mode))))

(event `EnhancedInput|/Game/2D_Game/Inputs/IA_Movement`
  (params (ActionValue :type "Vector2D Structure") (ElapsedSeconds :type "Float (double-precision)") (TriggeredSeconds :type "Float (double-precision)") (InputAction :type "InputAction Object Reference" :default "/Game/2D_Game/Inputs/IA_Movement.IA_Movement"))
  (:`Triggered`
    (if (not (`self.IsInteractionLocked`))
      (set `self.X_Direction` ActionValue_X)
      (set `self.Y_Direction` ActionValue_Y)
      (`self.AddMovementInput` (1.0 0.0 0.0) (`self.X_Direction`))
      (`self.AddMovementInput` (0.0 1.0 0.0) (`self.Y_Direction`)))))

(event `EnhancedInput|/Game/2D_Game/Inputs/IA_Interaction`
  (params (ActionValue :type Boolean) (ElapsedSeconds :type "Float (double-precision)") (TriggeredSeconds :type "Float (double-precision)") (InputAction :type "InputAction Object Reference" :default "/Game/2D_Game/Inputs/IA_Interaction.IA_Interaction"))
  (:`Started`
    (if (`self.IsInteractionLocked`)
      (if (`/Game/2D_Game/Widgets/WBP_NMDialogueBox.OngoingRevealing` (`/Game/2D_Game/Widgets/WBP_MainHUD.WBP_DialogueBox` (`/Game/2D_Game/Blueprints/2D_GameMode.HUDWidget` (`self.GameMode`))))
        (`/Game/2D_Game/Widgets/WBP_NMDialogueBox.InstaReveal` (`/Game/2D_Game/Widgets/WBP_MainHUD.WBP_DialogueBox` (`/Game/2D_Game/Blueprints/2D_GameMode.HUDWidget` (`self.GameMode`))))
        (else
          (bind _lastinteracted (`self.LastInteracted`)
            (:`then`
              (bind _hasnextline (message `/Game/2D_Game/Blueprints/Interfaces/BPI_Interaction.ShowNextLine` _lastinteracted))
              (if (not _hasnextline)
                (`self.EndInteraction`)
                (bind _lastinteracted_2 (`self.LastInteracted`)
                  (:`then`
                    (message `/Game/2D_Game/Blueprints/Interfaces/BPI_Interaction.FinishInteraction` _lastinteracted_2)
                    (set `self.LastInteracted` (`self.NullActor`))
                    (`/Game/2D_Game/Widgets/WBP_NMDialogueBox.HideDialogue` (`/Game/2D_Game/Widgets/WBP_MainHUD.WBP_DialogueBox` (`/Game/2D_Game/Blueprints/2D_GameMode.HUDWidget` (`self.GameMode`)))))
                  (:`else`))))
            (:`else`))))
      (else
        (for _array_element (`PrimitiveComponent.GetOverlappingActors` (`self.InteractCheck`) null)
          (`|ExecutionSequence`
            (:`then_0`
              (if (`KismetSystemLibrary.DoesImplementInterface` _array_element "/Game/2D_Game/Blueprints/Interfaces/BPI_Item.BPI_Item_C")
                (bind _itemname (message `/Game/2D_Game/Blueprints/Interfaces/BPI_Item.ItemPicked` _array_element))
                (`/Game/2D_Game/Blueprints/Inventory/BPC_Inventory.AddItemToInventory` (`self.BPC_Inventory`) _itemname)))
            (:`then_1`
              (if (!= _array_element self)
                (message `/Game/2D_Game/Blueprints/Interfaces/BPI_Interaction.Interact` _array_element self)
                (set `self.LastInteracted` _array_element)
                (break)))))
        (`KismetSystemLibrary.Delay` (`self.TimeToHideMsg`))
        (if (== (`Widget.GetVisibility` (`/Game/2D_Game/Widgets/WBP_MainHUD.WBP_MessageBox` (`/Game/2D_Game/Blueprints/2D_GameMode.HUDWidget` (`self.GameMode`)))) 0)
          (`/Game/2D_Game/Widgets/WBP_MainHUD.Hide Item Message` (`/Game/2D_Game/Blueprints/2D_GameMode.HUDWidget` (`self.GameMode`))))))))

(event `EnhancedInput|/Game/2D_Game/Inputs/IA_Inventory`
  (params (ActionValue :type Boolean) (ElapsedSeconds :type "Float (double-precision)") (TriggeredSeconds :type "Float (double-precision)") (InputAction :type "InputAction Object Reference" :default "/Game/2D_Game/Inputs/IA_Inventory.IA_Inventory"))
  (:`Started`
    (`/Game/2D_Game/Widgets/WBP_MainHUD.Toggle Inventory Visibility` (`/Game/2D_Game/Blueprints/2D_GameMode.HUDWidget` (`self.GameMode`)))))

(fn `EndInteraction`
  (set `self.IsInteractionLocked` false))

(fn `Interact`
  (params (Insitigator :type "/Game/2D_Game/Blueprints/Characters/MainCharacter/PlayerModel_BP Object Reference")))

(fn `ShowNextLine`
  (returns (HasNextLine :type Boolean))
  (return false))

(fn `StartInteraction`
  (set `self.IsInteractionLocked` true)
  (`MovementComponent.StopMovementImmediately` (`self.CharacterMovement`)))

(fn `UserConstructionScript`)