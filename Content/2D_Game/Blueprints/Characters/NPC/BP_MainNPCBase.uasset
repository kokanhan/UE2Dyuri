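; BP_MainNPCBase is the base Blueprint for main NPCs that hold data-driven dialogue in the 2D game.
; Interacting starts an interaction on both instigator and NPC, then shows the current DialogueDataTest1 row's speaker and text through the GameMode's HUD widget.
; ShowNextLine follows each row's NextRow link until it is empty, then resets to the starting row and returns false to signal the conversation's end.
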(event `/Game/2D_Game/Blueprints/Interfaces/BPI_Interaction.Interact`
  (params (Insitigator :type "/Game/2D_Game/Blueprints/Characters/MainCharacter/PlayerModel_BP Object Reference"))
  (`KismetSystemLibrary.PrintString` "call的是主npc的interact")
  (`/Game/2D_Game/Blueprints/Characters/MainCharacter/PlayerModel_BP.StartInteraction` Insitigator)
  (`self.StartInteraction`)
  (`self.ShowMainDialogue`))

(event `/Game/2D_Game/Blueprints/Interfaces/BPI_Interaction.FinishInteraction`)

(fn `GetWidgetType`
  (returns (WidgetType :type "/Game/2D_Game/Widgets/EWidgetType Enum"))
  (return "NewEnumerator2"))

(fn `ShowMainDialogue`
  (bind _returnvalue (`|GetDataTableRow` "/Game/2D_Game/DataTables/DialogueDataTest1.DialogueDataTest1" (`self.CurrentRowName`))
    (:`then`
      (`KismetSystemLibrary.PrintString` "call show main dialogue on npc 111")
      (bind (_dialoguetext _nextrow _dialoguenpcname) (break `/Game/2D_Game/DataTables/S_DialogueData` _returnvalue))
      (`/Game/2D_Game/Widgets/WBP_MainHUD.ShowMainDialogueOnHUD` (`/Game/2D_Game/Blueprints/2D_GameMode.HUDWidget` (`self.GameMode`)) self _dialoguenpcname _dialoguetext)
      (set `self.Next Row` _nextrow)
      (return))))

(fn `ShowNextLine`
  (returns (HasNextLine :type Boolean))
  (if (`KismetStringLibrary.IsEmpty` (`self.Next Row`))
    (set `self.CurrentRowName` (`self.ResetRowName`))
    (`KismetSystemLibrary.PrintString` "我得罪谁了")
    ;[1 1 1] 交互直到没有next line为止
    (return false)
    (else
      (set `self.CurrentRowName` (`KismetStringLibrary.Conv_StringToName` (`self.Next Row`)))
      (`KismetSystemLibrary.PrintString` "保佑我妈祖")
      (`self.ShowMainDialogue`)
      (return true))))

(fn `UserConstructionScript`
  (`parent.UserConstructionScript`))