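; Base RPG NPC character for a 2D game that players can interact with to hold data table-driven dialogue.
; Interacting notifies the instigator, locks the NPC, stops its movement, hides its dialogue indicator and sends the current row to the GameMode's HUD widget.
; ShowNextLine follows each row's NextRow link, resetting to the starting row when none remains.
; FinishInteraction unlocks the NPC and restores the indicator.
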(event `self.ReceiveBeginPlay`
  (set `self.ResetRowName` (`self.CurrentRowName`))
  (bind _as2d_game_mode (cast `/Game/2D_Game/Blueprints/2D_GameMode` (`GameplayStatics.GetGameMode`)))
  (set `self.GameMode` _as2d_game_mode))

(event `/Game/2D_Game/Blueprints/Interfaces/BPI_Interaction.FinishInteraction`
  (`self.EndInteraction`))

(event `/Game/2D_Game/Blueprints/Interfaces/BPI_Interaction.Interact`
  (params (Insitigator :type "/Game/2D_Game/Blueprints/Characters/MainCharacter/PlayerModel_BP Object Reference"))
  (`KismetSystemLibrary.PrintString` "call的是次要npc d的interact event")
  (`/Game/2D_Game/Blueprints/Characters/MainCharacter/PlayerModel_BP.StartInteraction` Insitigator)
  (`self.StartInteraction`)
  (`self.ShowDialogue`))

(fn `EndInteraction`
  (set `self.IsInteractionLocked` false)
  (`SceneComponent.SetVisibility` (`self.Widget_DialogueIndicator`) true false))

(fn `GetWidgetType`
  (returns (WidgetType :type "/Game/2D_Game/Widgets/EWidgetType Enum"))
  (return "NewEnumerator0"))

(fn `ShowDialogue`
  (bind _returnvalue (`|GetDataTableRow` "/Game/2D_Game/DataTables/DialogueDataTest1.DialogueDataTest1" (`self.CurrentRowName`))
    (:`then`
      (bind (_dialoguetext _nextrow _dialoguenpcname) (break `/Game/2D_Game/DataTables/S_DialogueData` _returnvalue))
      (`/Game/2D_Game/Widgets/WBP_MainHUD.ShowDialogueOnHUD` (`/Game/2D_Game/Blueprints/2D_GameMode.HUDWidget` (`self.GameMode`)) self _dialoguetext _dialoguenpcname)
      (set `self.Next Row` _nextrow)
      (return))))

(fn `ShowNextLine`
  (returns (HasNextLine :type Boolean))
  (if (`KismetStringLibrary.IsEmpty` (`self.Next Row`))
    (set `self.CurrentRowName` (`self.ResetRowName`))
    ;[1 1 1] 交互直到没有next line为止
    (return false)
    (else
      (set `self.CurrentRowName` (`KismetStringLibrary.Conv_StringToName` (`self.Next Row`)))
      (`self.ShowDialogue`)
      (return true))))

(fn `StartInteraction`
  (set `self.IsInteractionLocked` true)
  (`MovementComponent.StopMovementImmediately` (`self.CharacterMovement`))
  (`SceneComponent.SetVisibility` (`self.Widget_DialogueIndicator`) false false))

(fn `UserConstructionScript`)